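; FlyPawn is a free-flying player pawn driven by Enhanced Input with a visible mouse cursor.
; BeginPlay adds the keyboard and mouse mapping context, and movement inputs move the pawn along its forward, right and up vectors.
; Pitch and yaw look apply only while the right mouse input is active.
; Left click traces under the cursor, sends an OnMouseInteract message to the hit actor and prints its name.
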(event `self.ReceiveBeginPlay`
  (set `PlayerController.bShowMouseCursor` true (`GameplayStatics.GetPlayerController` 0))
  (`EnhancedInputSubsystemInterface.AddMappingContext` (pcsubsystem `EnhancedInputLocalPlayerSubsystem` (`GameplayStatics.GetPlayerController` 0)) "/Game/Input/IMC_Keyboard_Mouse.IMC_Keyboard_Mouse" 0 (struct)))

(event `EnhancedInput|/Game/Input/IA_Forward`
  (params (ActionValue :type "Float (double-precision)") (ElapsedSeconds :type "Float (double-precision)") (TriggeredSeconds :type "Float (double-precision)") (InputAction :type "InputAction Object Reference" :default "/Game/Input/IA_Forward.IA_Forward"))
  (:`Triggered`
    (`self.AddMovementInput` (`self.GetActorForwardVector`) ActionValue)))

(event `EnhancedInput|/Game/Input/IA_MoveRight`
  (params (ActionValue :type "Float (double-precision)") (ElapsedSeconds :type "Float (double-precision)") (TriggeredSeconds :type "Float (double-precision)") (InputAction :type "InputAction Object Reference" :default "/Game/Input/IA_MoveRight.IA_MoveRight"))
  (:`Triggered`
    (`self.AddMovementInput` (`self.GetActorRightVector`) ActionValue)))

(event `EnhancedInput|/Game/Input/IA_MoveUp`
  (params (ActionValue :type "Float (double-precision)") (ElapsedSeconds :type "Float (double-precision)") (TriggeredSeconds :type "Float (double-precision)") (InputAction :type "InputAction Object Reference" :default "/Game/Input/IA_MoveUp.IA_MoveUp"))
  (:`Triggered`
    (`self.AddMovementInput` (`self.GetActorUpVector`) ActionValue)))

(event `EnhancedInput|/Game/Input/IA_LookUp`
  (params (ActionValue :type "Float (double-precision)") (ElapsedSeconds :type "Float (double-precision)") (TriggeredSeconds :type "Float (double-precision)") (InputAction :type "InputAction Object Reference" :default "/Game/Input/IA_LookUp.IA_LookUp"))
  (:`Triggered`
    (if (`|GetInputActionValue`)
      (`self.AddControllerPitchInput` ActionValue))))

(event `EnhancedInput|/Game/Input/IA_Turn`
  (params (ActionValue :type "Float (double-precision)") (ElapsedSeconds :type "Float (double-precision)") (TriggeredSeconds :type "Float (double-precision)") (InputAction :type "InputAction Object Reference" :default "/Game/Input/IA_Turn.IA_Turn"))
  (:`Triggered`
    (if (`|GetInputActionValue`)
      (`self.AddControllerYawInput` ActionValue))))

(event `EnhancedInput|/Game/Input/IA_MouseLeft`
  (params (ActionValue :type Boolean) (ElapsedSeconds :type "Float (double-precision)") (TriggeredSeconds :type "Float (double-precision)") (InputAction :type "InputAction Object Reference" :default "/Game/Input/IA_MouseLeft.IA_MouseLeft"))
  (bind (_bblockinghit _binitialoverlap _time _distance _location _impactpoint _normal _impactnormal _physmat _hitactor) (`GameplayStatics.BreakHitResult` (`PlayerController.GetHitResultUnderCursorByChannel` (`GameplayStatics.GetPlayerController` 0) "TraceTypeQuery1" true)))
  (:`Started`
    (message `/Game/Blueprints/InterfaceTest/MouseHover.OnMouseInteract` _hitactor)
    (`KismetSystemLibrary.PrintString` (`KismetSystemLibrary.GetDisplayName` _hitactor))))

(fn `UserConstructionScript`)